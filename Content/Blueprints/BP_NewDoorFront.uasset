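; BP_NewDoorFront is an interactive door that swings and turns its handle when E is pressed inside a trigger box.
; Box overlap enables and disables the actor's input.
; Tick sets IsClosed from whether DoorRotation is negative, choosing between playing and reversing the door timeline.
; The handle timeline's Update plays the door timeline, whose Update applies handle pitch and door yaw from the two curves.
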(event OnComponentBeginOverlap(BoxCollison1)
  (params (OverlappedComponent :type Primitive%20Component%20Object%20Reference) (OtherActor :type Actor%20Object%20Reference) (OtherComp :type Primitive%20Component%20Object%20Reference) (OtherBodyIndex :type Integer) (bFromSweep :type Boolean) (SweepResult :type Hit%20Result%20Structure%20%28by%20ref%29))
  (Input|EnableInput (Game|GetPlayerController 0)))

(event OnComponentEndOverlap(BoxCollison1)
  (params (OverlappedComponent :type Primitive%20Component%20Object%20Reference) (OtherActor :type Actor%20Object%20Reference) (OtherComp :type Primitive%20Component%20Object%20Reference) (OtherBodyIndex :type Integer))
  (Input|DisableInput (Game|GetPlayerController 0)))

(event EventTick
  (params (DeltaSeconds :type Float%20%28single-precision%29))
  (Variables|Default|SetisClosed (< (stale Input|KeyboardEvents|E _doorrotation) 0.0)))

(event Input|KeyboardEvents|E
  (params (Key :type Key%20Structure :default "AnyKey"))
  (:Pressed
    (if (Variables|Default|GetisClosed)
      (bind _handlerotation (Timeline|HandleRotates Play)
        (:Update
          (bind _doorrotation (Timeline|DoorRotate Play)
            (:Update
              (Transformation|SetRelativeRotation (Variables|Default|GetSM_DoorHandleExt) (Math|Rotator|MakeRotator 0.0 _handlerotation 0.0) false false)
              (Transformation|SetRelativeRotation (Variables|Default|GetSM_Door201) (Math|Rotator|MakeRotator 0.0 0.0 _doorrotation) false false)))))
      (else
        (Timeline|DoorRotate Reverse)))))

(fn ConstructionScript)