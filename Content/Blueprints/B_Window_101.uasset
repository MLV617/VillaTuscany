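; Interactive window actor whose two parts, Winow01 and Window02, swing open and closed on the E key.
; Box overlap enables input for player controller 0, and leaving the box disables it.
; Two E handlers play or reverse separate yaw timelines based on the shared WinClosed flag.
; Tick derives that flag from Window02's timeline value, while an uncalled CustomEvent derives it from Winow01's.
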(event OnComponentBeginOverlap(Box)
  (params (OverlappedComponent :type Primitive%20Component%20Object%20Reference) (OtherActor :type Actor%20Object%20Reference) (OtherComp :type Primitive%20Component%20Object%20Reference) (OtherBodyIndex :type Integer) (bFromSweep :type Boolean) (SweepResult :type Hit%20Result%20Structure%20%28by%20ref%29))
  (Input|EnableInput (Game|GetPlayerController 0)))

(event OnComponentEndOverlap(Box)
  (params (OverlappedComponent :type Primitive%20Component%20Object%20Reference) (OtherActor :type Actor%20Object%20Reference) (OtherComp :type Primitive%20Component%20Object%20Reference) (OtherBodyIndex :type Integer))
  (Input|DisableInput (Game|GetPlayerController 0)))

(event Custom|CustomEvent
  (params (DeltaSeconds :type Float%20%28single-precision%29 :default 0.0))
  (Variables|Default|SetWinClosed (< (stale Input|KeyboardEvents|E _newtrack_0) 1.0)))

(event EventTick
  (params (DeltaSeconds :type Float%20%28single-precision%29))
  (Variables|Default|SetWinClosed (< (stale Input|KeyboardEvents|E _newtrack_1) 1.0)))

(event Input|KeyboardEvents|E
  (params (Key :type Key%20Structure :default "AnyKey"))
  (:Pressed
    (if (Variables|Default|GetWinClosed)
      (bind _newtrack_1 (Timeline|Window02rotation Play)
        (:Update
          (Transformation|SetRelativeRotation (Variables|Default|GetWindow02) (Math|Rotator|MakeRotator 0.0 0.0 _newtrack_1) false false)))
      (else
        (Timeline|Window02rotation Reverse)))))

(event Input|KeyboardEvents|E
  (params (Key :type Key%20Structure :default "AnyKey"))
  (:Pressed
    (if (Variables|Default|GetWinClosed)
      (bind _newtrack_0 (Timeline|WindowsRotation Play)
        (:Update
          (Transformation|SetRelativeRotation (Variables|Default|GetWinow01) (Math|Rotator|MakeRotator 0.0 0.0 _newtrack_0) false false)))
      (else
        (Timeline|WindowsRotation Reverse)))))

(fn ConstructionScript)