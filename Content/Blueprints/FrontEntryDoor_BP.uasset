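; Front entry door Blueprint that the player opens and closes with the E key while inside its trigger box.
; Overlap begin and end on the box enable and disable input for player controller 0, without checking the overlapping actor.
; E plays or reverses the DoorRotates timeline, which drives the door mesh's relative yaw.
; Tick derives IsClosed from whether the timeline's rotation value is below one, choosing the direction.
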(event OnComponentBeginOverlap(BoxCollision1)
  (params (OverlappedComponent :type Primitive%20Component%20Object%20Reference) (OtherActor :type Actor%20Object%20Reference) (OtherComp :type Primitive%20Component%20Object%20Reference) (OtherBodyIndex :type Integer) (bFromSweep :type Boolean) (SweepResult :type Hit%20Result%20Structure%20%28by%20ref%29))
  (Input|EnableInput (Game|GetPlayerController 0)))

(event OnComponentEndOverlap(BoxCollision1)
  (params (OverlappedComponent :type Primitive%20Component%20Object%20Reference) (OtherActor :type Actor%20Object%20Reference) (OtherComp :type Primitive%20Component%20Object%20Reference) (OtherBodyIndex :type Integer))
  (Input|DisableInput (Game|GetPlayerController 0)))

(event EventTick
  (params (DeltaSeconds :type Float%20%28single-precision%29))
  (Variables|Default|SetisClosed (< (stale Input|KeyboardEvents|E _dooropenrotate) 1.0)))

(event Input|KeyboardEvents|E
  (params (Key :type Key%20Structure :default "AnyKey"))
  (:Pressed
    (if (Variables|Default|GetisClosed)
      (bind _dooropenrotate (Timeline|DoorRotates Play)
        (:Update
          (Transformation|SetRelativeRotation (Variables|Default|GetSM_Door_201) (Math|Rotator|MakeRotator 0.0 0.0 _dooropenrotate) false false)))
      (else
        (Timeline|DoorRotates Reverse)))))

(fn ConstructionScript)